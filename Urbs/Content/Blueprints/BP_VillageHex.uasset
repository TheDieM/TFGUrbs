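; Village hex tile that accumulates wood, stone, iron, gold and population, and opens a village widget when clicked.
; TurnUpdate adds per-turn increments to each stock, while SetIncValues adjusts the resource increments.
; SetNeigborhoodvalues builds the neighborhood from the game mode's Tabletop and registers this village on adjacent land, mountain and sea hexes.
; Clicking clears the IsClose flag, blocking repeat widgets, and passes name, level and itself to WB_Village.
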(event `self.ReceiveActorOnClicked`
  (params (ButtonPressed :type "Key Structure"))
  (if (`self.isClose`)
    (set `self.isClose` false)
    (bind _returnvalue (`|CreateWidget` "/Game/Widgets/WB_Village.WB_Village_C"))
    (bind _output_get (set `self.Widget` _returnvalue))
    (`/Game/Widgets/WB_Village.setValues` _output_get (`self.Name`) (`KismetStringLibrary.Conv_IntToString` (`self.Level`)) self)
    (`UserWidget.AddToViewport` (`self.Widget`) 0)))

(fn `setIncValues`
  (params (incWood :type Integer) (incStone :type Integer) (incIron :type Integer) (incGold :type Integer))
  (set `self.incWood` (+ incWood (`self.incWood`)))
  (set `self.incStone` (+ incStone (`self.incStone`)))
  (set `self.incIron` (+ incIron (`local.incIron`)))
  (set `self.incGold` (+ incGold (`local.incGold`))))

(fn `SetNeigborhoodvalues`
  (locals (Index :type Integer) (item :type "Actor Object Reference"))
  (bind _returnvalue (`GameplayStatics.GetGameMode`))
  ;[1 1 1] Get Tabletop and Set Neighborhood
  (if (== (`GameplayStatics.GetObjectClass` _returnvalue) "/Game/Blueprints/BP_FirstPersonGameMode.BP_FirstPersonGameMode_C")
    (bind _asbp_first_person_game_mode (cast `/Game/Blueprints/BP_FirstPersonGameMode` _returnvalue))
    (`self.SetNeighborhood` (`/Game/Blueprints/BP_FirstPersonGameMode.Tabletop` _asbp_first_person_game_mode))
    ;[1 1 1] Set owner
    (for _array_element (`self.Neighborhood`)
      (bind _returnvalue_2 (`GameplayStatics.GetObjectClass` _array_element))
      (if (== _returnvalue_2 "/Game/Blueprints/BP_LandHex.BP_LandHex_C")
        (bind _asbp_land_hex (cast `/Game/Blueprints/BP_LandHex` _array_element))
        (`/Game/Blueprints/BP_LandHex.setVillage` _asbp_land_hex self)
        (elif (== _returnvalue_2 "/Game/Blueprints/BP_MountainHex.BP_MountainHex_C")
          (bind _asbp_mountain_hex (cast `/Game/Blueprints/BP_MountainHex` (`local.item`)))
          (`/Game/Blueprints/BP_MountainHex.setVillage` _asbp_mountain_hex self)
          (elif (== _returnvalue_2 "/Game/Blueprints/BP_SeaHex.BP_SeaHex_C")
            (bind _asbp_sea_hex (cast `/Game/Blueprints/BP_SeaHex` (`local.item`)))
            (`/Game/Blueprints/BP_SeaHex.setVillage` _asbp_sea_hex self)))))))

(fn `TurnUpdate`
  (set `self.Wood` (+ (`self.Wood`) (`self.incWood`)))
  (set `self.Stone` (+ (`self.Stone`) (`self.incStone`)))
  (set `self.Iron` (+ (`self.Iron`) (`self.incIron`)))
  (set `self.Gold` (+ (`self.Gold`) (`self.incGold`)))
  (set `self.Population` (+ (`self.Population`) (`self.incPopulation`))))

(fn `UserConstructionScript`)