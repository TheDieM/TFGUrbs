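; BP_Tabletop builds a tile grid of water, grass and mountain terrain using one instanced static mesh component per type.
; GenerateGrid clears all instances, calls IsRandomizeLayout, then loops over the Y and X cell counts.
; For each cell, GenerateVector supplies the location and GetHeight maps it to a height level that selects which mesh receives an instance.
; The construction script is empty, so generation runs only through the GenerateGrid event.
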(event `Clear Grid`
  (`InstancedStaticMeshComponent.ClearInstances` (`self.ISM_Water`))
  (`InstancedStaticMeshComponent.ClearInstances` (`self.ISM_Grass`))
  (`InstancedStaticMeshComponent.ClearInstances` (`self.ISM_Mountain`)))

(event `Generate Grid`
  (`self.Clear Grid`)
  (`self.isRandomizeLayout`)
  (bind _returnvalue (`self.GetYCellCount`))
  (for _index (range (+ _returnvalue 1))
    (bind _returnvalue_2 (`self.GetXCellCount`))
    (for _index_2 (range (+ _returnvalue_2 1))
      (bind _returnvalue_3 (`self.GenerateVector` _index_2 _index))
      (bind _returnvalue_4 (`self.GetHeight` _returnvalue_3))
      (if (== _returnvalue_4 1)
        (`InstancedStaticMeshComponent.AddInstance` (`self.ISM_Water`) (`KismetMathLibrary.MakeTransform` _returnvalue_3) false)
        (elif (== _returnvalue_4 2)
          (`InstancedStaticMeshComponent.AddInstance` (`self.ISM_Grass`) (`KismetMathLibrary.MakeTransform` _returnvalue_3) false)
          (elif (== _returnvalue_4 3)
            (`InstancedStaticMeshComponent.AddInstance` (`self.ISM_Mountain`) (`KismetMathLibrary.MakeTransform` _returnvalue_3) false)))))))

(fn `UserConstructionScript`)